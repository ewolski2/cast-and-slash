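; Big ghoul enemy character that growls at random intervals, attacks the player and drops gold on death.
; A looping timer toggles the anim blueprint's attack flag by player range.
; Hits on a non-blocking player deal damage after a delay and range recheck, gated by CanDealDmg.
; Taking damage flashes a dynamic material; death sets the animation flag, disables collision, stops movement, spawns random gold and later destroys the actor.
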(event Custom|TakeDamage
  (params (Damage :type Float%20%28double-precision%29))
  (bind _dynamicmat (Variables|Default|GetDynamicMat))
  (bind _dynamicmat_2 (Variables|Default|GetDynamicMat))
  ;[0.15 0.15 0.15 0.5] Take Damage
  (Audio|PlaySoundatLocation "/Game/DarkWav/Impact_Guts_Gore_01.Impact_Guts_Gore_01" (Transformation|GetActorLocation) "0, 0, 0" 1.0 1.0 0.0 0 0 0 0)
  (Variables|Default|SetHealth (- (Variables|Default|GetHealth) Damage))
  (Rendering|Material|SetVectorParameterValue _dynamicmat_2 "Albedo Tint" (Utilities|Struct|MakeLinearColor 1.0 0.0 0.0 1.0) :!class /Script/Engine.MaterialInstanceDynamic)
  (Rendering|Material|SetScalarParameterValue _dynamicmat_2 "Base Emissive" 0.15 :!class /Script/Engine.MaterialInstanceDynamic)
  (Utilities|FlowControl|Sequence
    (:then_0
      (Utilities|FlowControl|Delay 0.2)
      (Rendering|Material|SetVectorParameterValue _dynamicmat "Albedo Tint" (Utilities|Struct|MakeLinearColor 1.0 1.0 1.0 1.0) :!class /Script/Engine.MaterialInstanceDynamic)
      (Rendering|Material|SetScalarParameterValue _dynamicmat "Base Emissive" 2.0 :!class /Script/Engine.MaterialInstanceDynamic))
    (:then_1
      (if (<= (Variables|Default|GetHealth) 0.0)
        (bind _asabp_ghoul (Utilities|Casting|CastToABP_Ghoul (Components|SkeletalMesh|GetAnimInstance (Variables|Character|GetMesh))))
        (Variables|/Game/Assets/Ghoul/ABP_Ghoul.ABP_Ghoul_C|SetIsDead _asabp_ghoul true)
        (AI|Navigation|StopMovement (Pawn|GetController))
        (Collision|SetActorEnableCollision false)
        (Variables|Default|SetbUseControllerRotationYaw false)
        (Game|SpawnActorfromClass (Utilities|Select :Index (Math|Random|RandomIntegerinRange 0 1) :Option%200 "/Game/Interactable/Gold_big.Gold_big_C" :Option%201 "/Game/Interactable/Gold_small.Gold_small_C") (Math|Transform|MakeTransform (Transformation|GetWorldLocation (Variables|Default|Getgoldspawn)) "0, 0, 0" "1.000000,1.000000,1.000000") "Undefined" "MultiplyWithRoot" 0 0)
        (Utilities|FlowControl|Delay 15.0)
        (Actor|DestroyActor)))))

(event EventTick
  (params (DeltaSeconds :type Float%20%28single-precision%29))
  (bind _returnvalue (Transformation|GetActorLocation))
  (bind _output_get (Variables|Default|SetTimer (+ DeltaSeconds (Variables|Default|GetTimer))))
  (if (>= _output_get (Variables|Default|GetTimerMax))
    (if (> (Variables|Default|GetHealth) 0.0)
      (Variables|Default|SetTimer 0.0)
      (Variables|Default|SetTimerMax (Math|Conversions|ToFloat(Integer) (Math|Random|RandomIntegerinRange 4 8)))
      (switch int (Math|Random|RandomIntegerinRange 0 3)
        (:0
          (Audio|PlaySoundatLocation "/Game/monster_sounds/24_Sinister_Slumber_Growl.24_Sinister_Slumber_Growl" _returnvalue "0, 0, 0" 0.4 1.0 0.0 "/Game/monster_sounds/Attenuator.Attenuator" 0 0 0))
        (:1
          (Audio|PlaySoundatLocation "/Game/monster_sounds/23_Untethered_Growl.23_Untethered_Growl" _returnvalue "0, 0, 0" 0.4 1.0 0.0 "/Game/monster_sounds/Attenuator.Attenuator" 0 0 0))
        (:2
          (Audio|PlaySoundatLocation "/Game/monster_sounds/25_Warning_Growl.25_Warning_Growl" _returnvalue "0, 0, 0" 0.4 1.0 0.0 "/Game/monster_sounds/Attenuator.Attenuator" 0 0 0))
        (:3
          (Audio|PlaySoundatLocation "/Game/monster_sounds/22_Searching_Growl.22_Searching_Growl" _returnvalue "0, 0, 0" 0.4 1.0 0.0 "/Game/monster_sounds/Attenuator.Attenuator" 0 0 0))))))

(event Collision|EventHit
  (params (MyComp :type Primitive%20Component%20Object%20Reference) (Other :type Actor%20Object%20Reference) (OtherComp :type Primitive%20Component%20Object%20Reference) (bSelfMoved :type Boolean) (HitLocation :type Vector :default "0, 0, 0") (HitNormal :type Vector :default "0, 0, 0") (NormalImpulse :type Vector :default "0, 0, 0") (Hit :type Hit%20Result%20Structure%20%28by%20ref%29))
  (bind _returnvalue (Game|GetPlayerCharacter 0))
  (bind _returnvalue_2 (Game|GetPlayerCharacter 0))
  (bind _returnvalue_3 (Transformation|GetActorLocation))
  (bind _attackrange (Variables|Default|GetAttackRange))
  (bind _returnvalue_4 (Transformation|GetActorLocation _returnvalue))
  (bind _returnvalue_5 (Math|Vector|Distance(Vector) _returnvalue_4 _returnvalue_3))
  (bind _returnvalue_6 (<= _returnvalue_5 _attackrange))
  (bind _asbp_third_person_character (Utilities|Casting|CastToBP_ThirdPersonCharacter _returnvalue_2))
  (if (and (and (== Other _returnvalue_2) (Variables|Default|GetcanDealDmg)) (not (Variables|/Game/ThirdPerson/Blueprints/BP_ThirdPersonCharacter.BP_ThirdPersonCharacter_C|Getblocking _asbp_third_person_character)))
    (Variables|Default|SetcanDealDmg false)
    (Utilities|FlowControl|Delay 1.25)
    (Development|PrintString (Utilities|String|ToString(Boolean) _returnvalue_6))
    (if _returnvalue_6
      (Variables|/Game/ThirdPerson/Blueprints/BP_ThirdPersonCharacter.BP_ThirdPersonCharacter_C|Sethealth _asbp_third_person_character (- (Variables|/Game/ThirdPerson/Blueprints/BP_ThirdPersonCharacter.BP_ThirdPersonCharacter_C|Gethealth _asbp_third_person_character) (Variables|Default|GetDamage)))
      (switch int (Math|Random|RandomIntegerinRange 0 3)
        (:0
          (Audio|PlaySoundatLocation "/Game/damage_vocalization/11_TORAK_-_Damage_Grunt_D.11_TORAK_-_Damage_Grunt_D" (Transformation|GetActorLocation (Game|GetPlayerCharacter 0)) "0, 0, 0" 1.0 1.0 0.0 0 0 0 0))
        (:1
          (Audio|PlaySoundatLocation "/Game/damage_vocalization/07_NYKO_-_Damage_Grunt_D.07_NYKO_-_Damage_Grunt_D" (Transformation|GetActorLocation (Game|GetPlayerCharacter 0)) "0, 0, 0" 1.0 1.0 0.0 0 0 0 0))
        (:2
          (Audio|PlaySoundatLocation "/Game/damage_vocalization/02_REN_-_Damage_Grunt_B.02_REN_-_Damage_Grunt_B" (Transformation|GetActorLocation (Game|GetPlayerCharacter 0)) "0, 0, 0" 1.0 1.0 0.0 0 0 0 0))
        (:3
          (Audio|PlaySoundatLocation "/Game/damage_vocalization/19_TYR_-_Damage_Grunt_A.19_TYR_-_Damage_Grunt_A" (Transformation|GetActorLocation (Game|GetPlayerCharacter 0)) "0, 0, 0" 1.0 1.0 0.0 0 0 0 0))))
    (Variables|Default|SetcanDealDmg true)))

(event EventBeginPlay
  (bind _mesh (Variables|Character|GetMesh))
  (Utilities|Time|SetTimerbyFunctionName 0 "CheckAttackRange" 0.2 true)
  (bind _returnvalue (Rendering|Material|CreateDynamicMaterialInstance (Rendering|Material|GetMaterial _mesh 0) "None" "None" :!class /Script/Engine.KismetMaterialLibrary))
  (bind _output_get (Variables|Default|SetDynamicMat _returnvalue))
  (Rendering|Material|SetMaterial _mesh 0 _output_get)
  (Variables|Default|SetAIControllerClass "/Game/Characters/BP_GhoulAI.BP_GhoulAI_C")
  (Variables|Default|SetcanDealDmg true))

(fn ConstructionScript)

(fn CheckAttackRange
  (if (<= (Math|Vector|Distance(Vector) (Transformation|GetActorLocation (Game|GetPlayerCharacter 0)) (Transformation|GetActorLocation)) (Variables|Default|GetAttackRange))
    (bind _asabp_ghoul (Utilities|Casting|CastToABP_Ghoul (Components|SkeletalMesh|GetAnimInstance (Variables|Character|GetMesh))))
    (Variables|/Game/Assets/Ghoul/ABP_Ghoul.ABP_Ghoul_C|SetIsAttacking _asabp_ghoul true)
    (else
      (bind _asabp_ghoul_2 (Utilities|Casting|CastToABP_Ghoul (Components|SkeletalMesh|GetAnimInstance (Variables|Character|GetMesh))))
      (Variables|/Game/Assets/Ghoul/ABP_Ghoul.ABP_Ghoul_C|SetIsAttacking _asabp_ghoul_2 false))))

(fn DamageWindow
  (Variables|Default|SetcanDealDmg false)
  (Development|PrintString "Hello"))