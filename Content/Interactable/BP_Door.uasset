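; BP_Door is an interactable locked door that the player opens with the interact input when they hold a key.
; An Interact overlap component enables the door's input while the third-person character is inside it.
; With HasKey, a timeline swings the Hinge open by yaw while an opening sound plays and fades out at the end; otherwise the character shows a no-key message.
; The Opened flag gates interaction but is never set true here.
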(event OnComponentBeginOverlap(Interact)
  (params (OverlappedComponent :type Primitive%20Component%20Object%20Reference) (OtherActor :type Actor%20Object%20Reference) (OtherComp :type Primitive%20Component%20Object%20Reference) (OtherBodyIndex :type Integer) (bFromSweep :type Boolean) (SweepResult :type Hit%20Result%20Structure%20%28by%20ref%29))
  (Utilities|Casting|CastToBP_ThirdPersonCharacter OtherActor)
  (Input|EnableInput (Game|GetPlayerController 0)))

(event OnComponentEndOverlap(Interact)
  (params (OverlappedComponent :type Primitive%20Component%20Object%20Reference) (OtherActor :type Actor%20Object%20Reference) (OtherComp :type Primitive%20Component%20Object%20Reference) (OtherBodyIndex :type Integer))
  (Utilities|Casting|CastToBP_ThirdPersonCharacter OtherActor)
  (Input|DisableInput (Game|GetPlayerController 0)))

(event Input|EnhancedActionEvents|EnhancedInputActionIA_Interact
  (params (ActionValue :type Boolean) (ElapsedSeconds :type Float%20%28double-precision%29) (TriggeredSeconds :type Float%20%28double-precision%29) (InputAction :type Input%20Action%20Object%20Reference :default "/Game/Input/Actions/IA_Interact.IA_Interact"))
  (bind _door_opening_cue (Variables|Default|Getdoor-opening_cue))
  (if (not (Variables|Default|Getopened))
    (bind _asbp_third_person_character (Utilities|Casting|CastToBP_ThirdPersonCharacter (Game|GetPlayerCharacter 0)))
    (if (Variables|/Game/ThirdPerson/Blueprints/BP_ThirdPersonCharacter.BP_ThirdPersonCharacter_C|GethasKey _asbp_third_person_character)
      (Utilities|FlowControl|Sequence
        (:then_0
          (bind _alpha (Timeline|Timeline Play)
            (:Update
              (Transformation|SetRelativeRotation (Variables|Default|GetHinge) (Math|Rotator|MakeRotator 0.0 0.0 (* _alpha -9e+01)) false false))
            (:Finished
              (Audio|Components|Audio|FadeOut _door_opening_cue 0.0 0.0 "Linear" :!class /Script/Engine.AudioComponent))))
        (:then_1
          (Audio|Components|Audio|Play _door_opening_cue 0.0)))
      (else
        (Default|ShowNoKey _asbp_third_person_character)))))

(event EventBeginPlay
  (Variables|Default|Setopened false))

(event Collision|EventActorBeginOverlap
  (params (OtherActor :type Actor%20Object%20Reference)))

(event EventTick
  (params (DeltaSeconds :type Float%20%28single-precision%29)))

(fn ConstructionScript)