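; BP_Chest is an interactable chest that opens on input and holds a collectible coin.
; An overlap volume enables input only while the third-person character is inside.
; Interacting swings the lid open on a timeline with a sound, and a second handler collects the coin once the chest is marked open.
; When the collect sound finishes, the coin is destroyed and AddGold is called, though that function is empty.
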(event OnComponentBeginOverlap(Interact)
  (params (OverlappedComponent :type Primitive%20Component%20Object%20Reference) (OtherActor :type Actor%20Object%20Reference) (OtherComp :type Primitive%20Component%20Object%20Reference) (OtherBodyIndex :type Integer) (bFromSweep :type Boolean) (SweepResult :type Hit%20Result%20Structure%20%28by%20ref%29))
  (Utilities|Casting|CastToBP_ThirdPersonCharacter OtherActor)
  (Input|EnableInput (Game|GetPlayerController 0)))

(event OnComponentEndOverlap(Interact)
  (params (OverlappedComponent :type Primitive%20Component%20Object%20Reference) (OtherActor :type Actor%20Object%20Reference) (OtherComp :type Primitive%20Component%20Object%20Reference) (OtherBodyIndex :type Integer))
  (Utilities|Casting|CastToBP_ThirdPersonCharacter OtherActor)
  (Input|DisableInput (Game|GetPlayerController 0)))

(event OnAudioFinished(coin_collect)
  (Components|DestroyComponent (Variables|Default|Getcoin))
  (CallFunction|AddGold))

(event Input|EnhancedActionEvents|EnhancedInputActionIA_Interact
  (params (ActionValue :type Boolean) (ElapsedSeconds :type Float%20%28double-precision%29) (TriggeredSeconds :type Float%20%28double-precision%29) (InputAction :type Input%20Action%20Object%20Reference :default "/Game/Input/Actions/IA_Interact.IA_Interact"))
  (if (Variables|Default|GetbOpened)
    (if (Variables|Default|GetHasCoin)
      (Variables|Default|SetHasCoin false)
      (Audio|Components|Audio|Play (Variables|Default|Getcoin_collect) 0.0))))

(event Input|EnhancedActionEvents|EnhancedInputActionIA_Interact
  (params (ActionValue :type Boolean) (ElapsedSeconds :type Float%20%28double-precision%29) (TriggeredSeconds :type Float%20%28double-precision%29) (InputAction :type Input%20Action%20Object%20Reference :default "/Game/Input/Actions/IA_Interact.IA_Interact"))
  (bind _chest_opening_cue (Variables|Default|Getchest-opening_cue))
  (if (not (Variables|Default|GetbOpened))
    (Variables|Default|SetbOpened true)
    (Utilities|FlowControl|Sequence
      (:then_0
        (bind _alpha (Timeline|TL_OpenLid Play)
          (:Update
            (Transformation|SetRelativeRotation (Variables|Default|GetHinge) (Math|Rotator|MakeRotator (* _alpha -6e+01) 0.0 0.0) false false))
          (:Finished
            (Audio|Components|Audio|FadeOut _chest_opening_cue 0.0 0.0 "Linear" :!class /Script/Engine.AudioComponent))))
      (:then_1
        (Audio|Components|Audio|Play _chest_opening_cue 0.0)))))

(event EventBeginPlay
  (Variables|Default|SetbOpened false)
  (Variables|Default|SetHasCoin true))

(event Collision|EventActorBeginOverlap
  (params (OtherActor :type Actor%20Object%20Reference)))

(event EventTick
  (params (DeltaSeconds :type Float%20%28single-precision%29)))

(fn ConstructionScript)

(fn AddGold)