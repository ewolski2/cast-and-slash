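; BP_Merchant is an interactable shop NPC that opens an upgrade card shop for the player.
; On BeginPlay it creates a WBP_UpgradeCard widget, fills its random slots once and passes itself as owner.
; Its box overlap toggles input and plays hello or bye audio, removing the widget on exit.
; IA_Interact shows the shop with UI-only input and cursor, while CloseShop restores game-only input.
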(event OnComponentBeginOverlap(Box)
  (params (OverlappedComponent :type Primitive%20Component%20Object%20Reference) (OtherActor :type Actor%20Object%20Reference) (OtherComp :type Primitive%20Component%20Object%20Reference) (OtherBodyIndex :type Integer) (bFromSweep :type Boolean) (SweepResult :type Hit%20Result%20Structure%20%28by%20ref%29))
  (Utilities|Casting|CastToBP_ThirdPersonCharacter OtherActor)
  (Input|EnableInput (Game|GetPlayerController 0))
  (Audio|Components|Audio|Stop (Variables|Default|Getmerchant_bye_Cue))
  (Audio|Components|Audio|Play (Variables|Default|Getmerchant_hello_Cue) 0.0))

(event OnComponentEndOverlap(Box)
  (params (OverlappedComponent :type Primitive%20Component%20Object%20Reference) (OtherActor :type Actor%20Object%20Reference) (OtherComp :type Primitive%20Component%20Object%20Reference) (OtherBodyIndex :type Integer))
  (Utilities|Casting|CastToBP_ThirdPersonCharacter OtherActor)
  (Input|DisableInput (Game|GetPlayerController 0))
  (Audio|Components|Audio|Stop (Variables|Default|Getmerchant_hello_Cue))
  (Audio|Components|Audio|Play (Variables|Default|Getmerchant_bye_Cue) 0.0)
  (Widget|RemovefromParent (Variables|Components|GetShopWidget)))

(event Input|EnhancedActionEvents|EnhancedInputActionIA_Interact
  (params (ActionValue :type Boolean) (ElapsedSeconds :type Float%20%28double-precision%29) (TriggeredSeconds :type Float%20%28double-precision%29) (InputAction :type Input%20Action%20Object%20Reference :default "/Game/Input/Actions/IA_Interact.IA_Interact"))
  (bind _returnvalue (Game|GetPlayerController 0))
  (bind _shopwidget (Variables|Components|GetShopWidget))
  (UserInterface|Viewport|AddtoViewport _shopwidget 0)
  (Input|SetInputModeUIOnly _returnvalue _shopwidget "DoNotLock" false)
  (Variables|/Script/Engine.PlayerController|SetbShowMouseCursor _returnvalue true))

(event EventBeginPlay
  (bind _returnvalue (UserInterface|CreateWidget "/Game/Interactable/WBP_UpgradeCard.WBP_UpgradeCard_C"))
  (bind _output_get (Variables|Components|SetShopWidget _returnvalue))
  (Default|SetupRandomSlots _output_get)
  (Variables|/Game/Interactable/WBP_UpgradeCard.WBP_UpgradeCard_C|SetOwnerMerchant _output_get self))

(event Collision|EventActorBeginOverlap
  (params (OtherActor :type Actor%20Object%20Reference)))

(event EventTick
  (params (DeltaSeconds :type Float%20%28single-precision%29)))

(fn ConstructionScript)

(fn CloseShop
  (bind _returnvalue (Game|GetPlayerController 0))
  (Widget|RemovefromParent (Variables|Components|GetShopWidget))
  (Input|SetInputModeGameOnly _returnvalue false)
  (Variables|/Script/Engine.PlayerController|SetbShowMouseCursor _returnvalue false))